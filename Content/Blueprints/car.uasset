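; A car actor that slides its static mesh along the world Y axis when play begins.
; BeginPlay stores the actor's location as Start, then plays a timeline whose track drives a vector lerp from Start to Start offset by End's Y component.
; Each update sets the mesh's world location directly, without sweep, so it does no collision checks along the path.
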(event `self.ReceiveBeginPlay`
  ;[1 1 1] Move vehicle -- src: https://www.youtube.com/watch?v=j5AM1Az7e0g
  (set `self.start` (`self.K2_GetActorLocation`))
  (bind (_direction _newtrack_0) (`Timeline|Timeline_0`)
    (:`Update`
      (`SceneComponent.K2_SetWorldLocation` (`self.StaticMesh`) (`KismetMathLibrary.VLerp` (`self.start`) (+ (`self.start`) (`KismetMathLibrary.MakeVector` 0.0 (.y (`self.end`)))) _newtrack_0) false false))))

(fn `UserConstructionScript`)